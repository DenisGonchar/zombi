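; Skeleton enemy AI character with light and heavy melee attacks, health, death and a random chance to drop an item.
; Attacks play random montages, sphere-trace on an "Attack" notify to damage Player-tagged actors, and toggle attack and movement flags exposed through getters.
; Damage feeds TDAHealth; death unpossesses the controller, triggers any drop, plays a montage, ragdolls on blend-out and expires.
; Stun and damage-number logic exist but are never triggered.
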(event `self.TDAHealth.OnHealthChange`
  (params (Health :type "Float (single-precision)") (Damage :type "Float (single-precision)"))
  (if (`self.IsDead`)
    _
    (elif false
      _)))

(event `self.TDAHealth.OnDead`
  (bind _deadanim (`self.DeadAnim`))
  (if (not (`self.IsDead`))
    (`self.DeadEvent`)
    (`|PlayMontage` (`self.Mesh`) (`|GetArrayItem` _deadanim (`KismetMathLibrary.RandomInteger` (`KismetArrayLibrary.Array_Length` _deadanim)))
      (:`then`
        (`PrimitiveComponent.SetCollisionEnabled` (`self.CapsuleComponent`) "NoCollision"))
      (:`OnBlendOut`
        (`PrimitiveComponent.SetSimulatePhysics` (`self.Mesh`) true)
        (`PrimitiveComponent.SetCollisionProfileName` (`self.Mesh`) "PhysicsActor" true)
        (`PrimitiveComponent.SetCollisionResponseToChannel` (`self.CapsuleComponent`) "ECC_Pawn" "ECR_Ignore")
        (`PrimitiveComponent.SetCollisionEnabled` (`self.Mesh`) "PhysicsOnly")))))

(event `self.ReceiveTick`
  (params (DeltaSeconds :type "Float (single-precision)")))

(event `self.ReceiveAnyDamage`
  (params (Damage :type "Float (single-precision)") (DamageType :type "DamageType Object Reference") (InstigatedBy :type "Controller Object Reference") (DamageCauser :type "Actor Object Reference"))
  (if (not (`self.IsDead`))
    (`TDAHealthComponent.ChangeHealthValue` (`self.TDAHealth`) (* Damage -1.0))))

(event `self.ReceiveBeginPlay`
  (if (> (`KismetMathLibrary.RandomFloat`) 0.7)
    (bind _returnvalue (`AddComponent|NODE_AddBP_DropItomComponent-0`))
    (set `self.DropComponent` _returnvalue)))

(event `/Game/Blueprint/NPS_Character/ZombiePawn/BPI_Combat.MeleeAttackLight`
  (bind _lightattackanim (`self.LightAttackAnim`))
  (bind _baselightdamage (`self.BaseLightDamage`))
  (`self.SetStateAttake` false)
  (bind _notifyname (`|PlayMontage` (`self.Mesh`) (`|GetArrayItem` _lightattackanim (`KismetMathLibrary.RandomInteger` (`KismetArrayLibrary.Array_Length` _lightattackanim))))
    (:`OnCompleted`
      (`self.SetStateAttake` true :!label _label))
    (:`OnInterrupted`
      (goto _label))
    (:`OnNotifyBegin`
      (if (== _notifyname "Attack")
        (bind _outhit (`KismetSystemLibrary.SphereTraceSingle` (+ (* (`self.GetActorForwardVector`) 100.0) (`self.K2_GetActorLocation`)) (+ (`self.K2_GetActorLocation`) (* (`self.GetActorForwardVector`) 200.0)) (`self.LightRadius`) "TraceTypeQuery4" false (`|MakeArray` self :!type "Actor Object Reference") "ForDuration"))
        (bind (_bblockinghit _binitialoverlap _time _distance _location _impactpoint _normal _impactnormal _physmat _hitactor) (`GameplayStatics.BreakHitResult` _outhit))
        (`/Engine/EditorBlueprintResources/StandardMacros.IsValid` _hitactor
          (:`Is Valid`
            (if (`self.ActorHasTag` _hitactor "Player")
              (`GameplayStatics.ApplyDamage` _hitactor (`KismetMathLibrary.RandomFloatInRange` (+ _baselightdamage 10.0) (- _baselightdamage 5.0)) (`self.GetController`) self))))))))

(event `/Game/Blueprint/NPS_Character/ZombiePawn/BPI_Combat.MeleeAttackHeavy`
  (bind _baseheavydamage (`self.BaseHeavyDamage`))
  (bind _heacyattackanim (`self.HeacyAttackAnim`))
  (`self.SetStateAttake` false)
  (`self.SetStateMovement` false)
  (bind _notifyname (`|PlayMontage` (`self.Mesh`) (`|GetArrayItem` _heacyattackanim (`KismetMathLibrary.RandomInteger` (`KismetArrayLibrary.Array_Length` _heacyattackanim))))
    (:`OnCompleted`
      (`self.SetStateMovement` true)
      (goto _label))
    (:`OnNotifyBegin`
      (if (== _notifyname "Attack")
        (bind _outhit (`KismetSystemLibrary.SphereTraceSingle` (+ (* (`self.GetActorForwardVector`) 100.0) (`self.K2_GetActorLocation`)) (+ (`self.K2_GetActorLocation`) (* (`self.GetActorForwardVector`) 200.0)) (`self.HealyRadius`) "TraceTypeQuery4" false (`|MakeArray` self :!type "Actor Object Reference") "ForDuration"))
        (bind (_bblockinghit _binitialoverlap _time _distance _location _impactpoint _normal _impactnormal _physmat _hitactor) (`GameplayStatics.BreakHitResult` _outhit))
        (`/Engine/EditorBlueprintResources/StandardMacros.IsValid` _hitactor
          (:`Is Valid`
            (if (`self.ActorHasTag` _hitactor "Player")
              (`GameplayStatics.ApplyDamage` _hitactor (`KismetMathLibrary.RandomFloatInRange` (+ _baseheavydamage 50.0) (- _baseheavydamage 10.0)) (`self.GetController`) self))))))))

(fn `CanAttack`
  (returns (bIsCanAttack :type Boolean))
  (return (`self.CanAttake`)))

(fn `CanMovement`
  (returns (bIsCanMove :type Boolean))
  (return (`self.CanMove`)))

(fn `DeadEvent`
  (bind _dropcomponent (`self.DropComponent`))
  (`Controller.UnPossess` (`self.GetController`))
  (`self.SetLifeSpan` 2.0)
  (`self.SetStateMovement` false)
  (`self.SetStateAttake` false)
  (set `self.IsDead` true)
  (`/Engine/EditorBlueprintResources/StandardMacros.IsValid` _dropcomponent
    (:`Is Valid`
      (`/Game/Blueprint/BP_DropItomComponent.Drop` _dropcomponent))))

(fn `Destroy Actor`
  (`self.K2_DestroyActor`))

(fn `SetStateAttake`
  (params (CanAttake :type Boolean))
  (set `self.CanAttake` CanAttake))

(fn `SetStateMovement`
  (params (CanMove :type Boolean))
  (set `self.CanMove` CanMove))

(fn `StunEnable`
  (`self.SetStateMovement` false)
  (`KismetSystemLibrary.K2_SetTimer` null "StunTime" (`self.StunTimer`))
  (`self.PlayAnimMontage` "/Game/Blueprint/Character/Animations/ThirdPersonIdle_Montage.ThirdPersonIdle_Montage")
  (set `CharacterMovementComponent.MaxWalkSpeed` 0.0 (`self.CharacterMovement`)))

(fn `StunTime`
  (`self.SetStateMovement` true)
  (set `CharacterMovementComponent.MaxWalkSpeed` 400.0 (`self.CharacterMovement`)))

(fn `UserConstructionScript`)