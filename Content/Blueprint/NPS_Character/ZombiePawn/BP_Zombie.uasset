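; BP_Zombie is an enemy character that chases the first BP_Character found, reissuing AI MoveTo every Tick while movement is allowed.
; Damage feeds the TDAHealth component, whose death event unpossesses it, plays a random death montage into ragdoll and sets a despawn lifespan.
; BeginPlay randomly adds a drop component that releases on death.
; Stun and floating damage-number logic exist but are disconnected.
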(event `self.TDAHealth.OnHealthChange`
  (params (Health :type "Float (single-precision)") (Damage :type "Float (single-precision)"))
  (if (`self.IsDead`)
    _
    (elif false
      _)))

(event `self.TDAHealth.OnDead`
  (if (not (`self.IsDead`))
    (`self.DeadEvent`)
    (`|PlayMontage` (`self.Mesh`) (select `bool` (> (`KismetMathLibrary.RandomFloat`) 0.5) :`false` "/Game/Blueprint/NPS_Character/AnimNPS/AM_Zombie_Death_1.AM_Zombie_Death_1" :`true` "/Game/Blueprint/NPS_Character/AnimNPS/AM_Zombie_Death_2.AM_Zombie_Death_2" :!type "AnimMontage Object Reference")
      (:`then`
        (`PrimitiveComponent.SetCollisionEnabled` (`self.CapsuleComponent`) "NoCollision"))
      (:`OnBlendOut`
        (`PrimitiveComponent.SetSimulatePhysics` (`self.Mesh`) true)
        (`PrimitiveComponent.SetCollisionProfileName` (`self.Mesh`) "PhysicsActor" true)
        (`PrimitiveComponent.SetCollisionResponseToChannel` (`self.CapsuleComponent`) "ECC_Pawn" "ECR_Ignore")
        (`PrimitiveComponent.SetCollisionEnabled` (`self.Mesh`) "PhysicsOnly")))))

(event `self.ReceiveTick`
  (params (DeltaSeconds :type "Float (single-precision)"))
  (bind _outactors (`GameplayStatics.GetAllActorsOfClass` "/Game/Blueprint/Character/BP_Character.BP_Character_C"))
  (bind _output (`|GetArrayItem` _outactors))
  (`/Engine/EditorBlueprintResources/StandardMacros.IsValid` _output
    (:`Is Valid`
      (if (`self.CanMove`)
        (`|AIMoveTo` (`self.GetController`) self (0.0 0.0 0.0) _output 20.0)))))

(event `self.ReceiveAnyDamage`
  (params (Damage :type "Float (single-precision)") (DamageType :type "DamageType Object Reference") (InstigatedBy :type "Controller Object Reference") (DamageCauser :type "Actor Object Reference"))
  (if (not (`self.IsDead`))
    (`TDAHealthComponent.ChangeHealthValue` (`self.TDAHealth`) (* Damage -1.0))))

(event `self.ReceiveBeginPlay`
  (if (> (`KismetMathLibrary.RandomFloat`) 0.7)
    (bind _returnvalue (`AddComponent|NODE_AddBP_DropItomComponent-0`))
    (set `self.DropComponent` _returnvalue)))

(fn `DeadEvent`
  (bind _dropcomponent (`self.DropComponent`))
  (`Controller.UnPossess` (`self.GetController`))
  (`self.SetLifeSpan` 10.0)
  (`self.SetStateMovement` false)
  (`self.SetStateAttake` false)
  (set `self.IsDead` true)
  (`/Engine/EditorBlueprintResources/StandardMacros.IsValid` _dropcomponent
    (:`Is Valid`
      (`/Game/Blueprint/BP_DropItomComponent.Drop` _dropcomponent))))

(fn `Destroy Actor`
  (`self.K2_DestroyActor`))

(fn `SetStateAttake`
  (params (CanAttake :type Boolean))
  (set `self.CanAttake` CanAttake))

(fn `SetStateMovement`
  (params (CanMove :type Boolean))
  (set `self.CanMove` CanMove))

(fn `StunEnable`
  (`self.SetStateMovement` false)
  (`KismetSystemLibrary.K2_SetTimer` null "StunTime" (`self.StunTimer`))
  (`self.PlayAnimMontage` "/Game/Blueprint/Character/Animations/ThirdPersonIdle_Montage.ThirdPersonIdle_Montage")
  (set `CharacterMovementComponent.MaxWalkSpeed` 0.0 (`self.CharacterMovement`)))

(fn `StunTime`
  (`self.SetStateMovement` true)
  (set `CharacterMovementComponent.MaxWalkSpeed` 400.0 (`self.CharacterMovement`)))

(fn `UserConstructionScript`)