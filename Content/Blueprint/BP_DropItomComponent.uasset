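; Actor component that makes its owner drop a random pickup when its Drop event is called.
; A coin flip selects either DropAmmo, which spawns rifle ammo, or DropFirst, which spawns a PickUpActor_First.
; Each spawns at the owner's location, lowered by a fixed height per item type.
; The component then destroys itself.
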(event `self.ReceiveTick`
  (params (DeltaSeconds :type "Float (single-precision)")))

(event `Drop`
  (if (> (`KismetMathLibrary.RandomFloat`) 0.5)
    (`self.DropAmmo`)
    (`self.K2_DestroyComponent`)
    (else
      (`self.DropFirst`)
      (`self.K2_DestroyComponent`))))

(fn `DropAmmo`
  (bind (_returnvalue_x _returnvalue_y _returnvalue_z) (`KismetMathLibrary.BreakVector` (`Actor.K2_GetActorLocation` (`self.GetOwner`))))
  (`|SpawnActorFromClass` "/Game/Blueprint/InteractionEnvironment/DropActor/drop_Ammo_Rifle.drop_Ammo_Rifle_C" (`KismetMathLibrary.MakeTransform` (`KismetMathLibrary.MakeVector` _returnvalue_x _returnvalue_y (- _returnvalue_z 90.0))) "Undefined" "OverrideRootScale" null null))

(fn `DropFirst`
  (bind (_returnvalue_x _returnvalue_y _returnvalue_z) (`KismetMathLibrary.BreakVector` (`Actor.K2_GetActorLocation` (`self.GetOwner`))))
  (`|SpawnActorFromClass` "/Game/Blueprint/InteractionEnvironment/DropActor/PickUpActor_First.PickUpActor_First_C" (`KismetMathLibrary.MakeTransform` (`KismetMathLibrary.MakeVector` _returnvalue_x _returnvalue_y (- _returnvalue_z 45.0))) "Undefined" "OverrideRootScale" null null))