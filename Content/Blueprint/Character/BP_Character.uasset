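; Character Blueprint that links weapon actions to animation and brings up the end-game screen.
; BeginPlay caches the BP_AnimBP instance, which receives the fire, reload-start and reload-end weapon events.
; Tick prints the current weapon's firing, reloading and round state as on-screen debug text.
; On unpossess under BP_GameMode, it adds the BPW_EndGame widget to the viewport and shows the mouse cursor.
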(event `self.ReceiveBeginPlay`
  (bind _asbp_anim_bp (cast `/Game/Blueprint/Character/BP_AnimBP` (`SkeletalMeshComponent.GetAnimInstance` (`self.Mesh`))))
  (set `self.As BP Anim BP` _asbp_anim_bp))

(event `self.ReceiveTick`
  (params (DeltaSeconds :type "Float (single-precision)"))
  (bind _returnvalue (`self.GetCurrentWeapon`))
  (`/Engine/EditorBlueprintResources/StandardMacros.IsValid` _returnvalue
    (:`Is Valid`
      (bind _returnvalue_2 (`WeaponDefault.GetWeaponRound` _returnvalue))
      (`KismetSystemLibrary.PrintString` (`KismetStringLibrary.Concat_StrStr` "Firing = " (`KismetStringLibrary.Conv_BoolToString` (`WeaponDefault.WeaponFiring` _returnvalue)) "   Rrload = " (`KismetStringLibrary.Conv_BoolToString` (`WeaponDefault.WeaponReloading` _returnvalue)) "    Reload = " (`KismetStringLibrary.Conv_IntToString` _returnvalue_2)) true true (struct :`G` 0.66 :`B` 1.0 :`A` 1.0) 0.001))))

(event `self.WeaponFireStart_BP`
  (params (Anim :type "AnimMontage Object Reference"))
  (`/Game/Blueprint/Character/BP_AnimBP.Fire` (`self.As BP Anim BP`) Anim))

(event `self.WeaponReloadStart_BP`
  (params (Anim :type "AnimMontage Object Reference"))
  (`/Game/Blueprint/Character/BP_AnimBP.Reload` (`self.As BP Anim BP`) Anim))

(event `self.WeaponReloadEnd_BP`
  (params (bIsSuccess :type Boolean))
  (`/Game/Blueprint/Character/BP_AnimBP.ReloadEnd` (`self.As BP Anim BP`) bIsSuccess))

(event `self.ReceiveUnpossessed`
  (params (OldController :type "Controller Object Reference"))
  (cast `/Game/Blueprint/Game/BP_GameMode` (`GameplayStatics.GetGameMode`))
  (bind _returnvalue (`|CreateWidget` "/Game/Blueprint/Widget/Blueprint/Widget/BPW_EndGame.BPW_EndGame_C"))
  (`UserWidget.AddToViewport` _returnvalue 0)
  (set `PlayerController.bShowMouseCursor` true (`GameplayStatics.GetPlayerController` 0)))

(fn `UserConstructionScript`)