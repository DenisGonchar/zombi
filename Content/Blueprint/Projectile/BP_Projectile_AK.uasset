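; BP_Projectile_AK is the AK weapon's projectile, a child Blueprint that sets up its Niagara trace effect when spawned.
; On BeginPlay it runs the parent logic, then casts player 0's pawn to BP_Character and gets the current weapon.
; It passes that weapon's fire end location to the Niagara TraceEnd parameter once, with no per-tick or overlap logic of its own.
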(event `self.ReceiveBeginPlay`
  (`parent.ReceiveBeginPlay`)
  (bind _asbp_character (cast `/Game/Blueprint/Character/BP_Character` (`GameplayStatics.GetPlayerPawn` 0)))
  (bind _returnvalue (`TDACharacter.GetCurrentWeapon` _asbp_character))
  (`FXSystemComponent.SetVectorParameter` (`self.Niagara`) "TraceEnd" (`WeaponDefault.GetFireEndLocation` _returnvalue)))

(fn `UserConstructionScript`
  (`parent.UserConstructionScript`))